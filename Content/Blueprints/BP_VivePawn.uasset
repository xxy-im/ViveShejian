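; VR pawn for bow-and-arrow shooting, which spawns a bow in the left hand at BeginPlay.
; Right shoulder spawns an arrow in the right hand or drops it with physics when not aiming.
; With an arrow on the bow, holding right trigger runs a Gate/RetriggerableDelay loop mapping hand distance to haptics and draw Strength.
; Releasing while aiming launches the arrow along the bow's ArrowForward, its speed scaled by hand distance.
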(event `SpawnBowAttachToLeftHand`
  (bind _left_hand (`self.Left Hand`))
  (bind _returnvalue (`|SpawnActorFromClass` "/Game/Blueprints/BP_Bow.BP_Bow_C" (`self.SpawnTransform`) "Undefined" "OverrideRootScale"))
  (set `self.BP_Bow` _returnvalue)
  (`self.K2_AttachToComponent` _returnvalue _left_hand "None" "KeepRelative" "KeepRelative" "KeepRelative" true)
  (`SceneComponent.SetHiddenInGame` _left_hand true false))

(event `self.ReceiveBeginPlay`
  (`self.SpawnBowAttachToLeftHand`))

(event `Key|MotionController_Right_Shoulder`
  (params (Key :type "Key Structure" :default "AnyKey"))
  (:`Pressed`
    (if (`self.bIsArrowAttached`)
      (if (not (`self.bIsAiming`))
        (`/Engine/EditorBlueprintResources/StandardMacros.IsValid` (`self.BP_Arrow`)
          (:`Is Valid`
            (`self.DropArrow`))))
      (else
        (`self.SpawnArrowAttachToRightHand`)))))

(event `SpawnArrowAttachToRightHand`
  (bind _right_hand (`self.Right Hand`))
  (bind _returnvalue (`|SpawnActorFromClass` "/Game/Blueprints/BP_Arrow.BP_Arrow_C" (`KismetMathLibrary.MakeTransform` (0.0 0.0 0.0) (struct :`Pitch` 90.0)) "Undefined" "OverrideRootScale"))
  (set `self.BP_Arrow` _returnvalue)
  (`self.K2_AttachToComponent` _returnvalue _right_hand "None" "KeepRelative" "KeepRelative" "KeepRelative" true)
  (`SceneComponent.SetHiddenInGame` _right_hand true false)
  (set `self.bIsArrowAttached` true))

(event `Key|MotionController_Right_Trigger`
  (params (Key :type "Key Structure" :default "AnyKey"))
  (:`Pressed`
    (set `self.bRightTrigerPressed` true)
    (`|ExecutionSequence`
      (:`then_0`
        (goto _label :!via `Open`))
      (:`then_1`
        (`/Engine/EditorBlueprintResources/StandardMacros.Gate` true :!label _label
          (:`Exit`
            (`|ExecutionSequence`
              (:`then_0`
                (if (`self.bIsArrowAttachedToBow`)
                  (`self.ReadyingShoot`)))
              (:`then_1`
                (`KismetSystemLibrary.RetriggerableDelay` 0.01)
                (goto _label))))))))
  (:`Released`
    (set `self.bRightTrigerPressed` false)
    (`|ExecutionSequence`
      (:`then_0`
        (goto _label :!via `Close`))
      (:`then_1`
        (`self.Shoot`)))))

(event `DropArrow`
  (bind _bp_arrow (`self.BP_Arrow`))
  (`self.K2_DetachFromActor` _bp_arrow "KeepWorld" "KeepRelative" "KeepWorld")
  (`PrimitiveComponent.SetSimulatePhysics` (`/Game/Blueprints/BP_Arrow.ArrowMesh` _bp_arrow) true)
  (`SceneComponent.SetHiddenInGame` (`self.Right Hand`) false false)
  (set `self.bIsArrowAttached` false))

(event `ReadyingShoot`
  (bind _distance (`self.GetHandDistance`))
  (`|ExecutionSequence`
    (:`then_0`
      (`PlayerController.PlayDynamicForceFeedback` (`GameplayStatics.GetPlayerController` 0) (`KismetMathLibrary.MapRangeClamped` _distance 10.0 90.0 0.0 0.5) 0.05 false false true true))
    (:`then_1`
      (set `self.Strength` (- (`KismetMathLibrary.MapRangeClamped` _distance 10.0 90.0 30.0 70.0) 30.0))
      (set `self.bIsAiming` true))))

(event `Shoot`
  (bind _bp_arrow (`self.BP_Arrow`))
  (bind _projectilemovement (`/Game/Blueprints/BP_Arrow.ProjectileMovement` _bp_arrow))
  (if (`self.bIsAiming`)
    (`self.K2_DetachFromActor` _bp_arrow "KeepWorld" "KeepWorld" "KeepWorld")
    (`ActorComponent.SetActive` _projectilemovement true false)
    (set `MovementComponent.Velocity` (* (`KismetMathLibrary.GreaterGreater_VectorRotator` (1.0 0.0 0.0) (`SceneComponent.K2_GetComponentRotation` (`/Game/Blueprints/BP_Bow.ArrowForward` (`self.BP_Bow`)))) (`KismetMathLibrary.MapRangeClamped` (`self.GetHandDistance`) 10.0 90.0 1000.0 2000.0)) _projectilemovement)
    (set `self.bIsAiming` false)
    (set `self.Strength` 0.0)
    (set `self.bIsArrowAttachedToBow` false)
    (`SceneComponent.SetHiddenInGame` (`self.Right Hand`) false false)
    (set `self.bIsArrowAttached` false)))

(fn `GetHandDistance`
  (returns (Distance :type "Float (double-precision)"))
  (return (`KismetMathLibrary.VSize` (- (`SceneComponent.K2_GetComponentLocation` (`self.Right Hand`)) (`SceneComponent.K2_GetComponentLocation` (`self.Left Hand`))))))

(fn `UserConstructionScript`)